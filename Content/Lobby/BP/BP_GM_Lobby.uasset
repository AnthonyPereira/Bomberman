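; BP_GM_Lobby is the lobby game mode that tracks connected lobby player controllers and the player count.
; When a new player starts, it adds the BP_PC_Lobby to an array, waits briefly, then calls HUDLobby on that controller.
; On logout it removes the controller; both paths pass the array length to BP_GS_Lobby through UpdatePlayers.
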(event EventHandleStartingNewPlayer
  (params (NewPlayer :type Player%20Controller%20Object%20Reference))
  (bind _asbp_pc_lobby (Utilities|Casting|CastToBP_PC_Lobby NewPlayer))
  (Utilities|Array|Add (Variables|Default|GetAllPC) _asbp_pc_lobby)
  (Utilities|FlowControl|Delay 0.2)
  (Default|HUD-Lobby _asbp_pc_lobby)
  (bind _asbp_gs_lobby (Utilities|Casting|CastToBP_GS_Lobby (Game|GetGameState)))
  (Default|UpdatePlayers _asbp_gs_lobby (Utilities|Array|Length (Variables|Default|GetAllPC))))

(event EventOnLogout
  (params (ExitingController :type Controller%20Object%20Reference))
  (bind _asbp_pc_lobby (Utilities|Casting|CastToBP_PC_Lobby ExitingController))
  (Utilities|Array|RemoveItem (Variables|Default|GetAllPC) _asbp_pc_lobby)
  (bind _asbp_gs_lobby (Utilities|Casting|CastToBP_GS_Lobby (Game|GetGameState)))
  (Default|UpdatePlayers _asbp_gs_lobby (Utilities|Array|Length (Variables|Default|GetAllPC))))

(fn ConstructionScript)