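; Podium actor that holds four mesh components and lets their materials be swapped individually by index.
; BeginPlay fills a List array with components 1 through 4 in order.
; Change Mesh looks up the entry at the given index and sets its first material slot to the supplied material, leaving the mesh itself unchanged.
; Overlap, Tick and construction logic are empty.
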(event EventBeginPlay
  (bind _list (Variables|Default|GetList))
  (Utilities|Array|Add _list (Variables|Default|Get1))
  (Utilities|Array|Add _list (Variables|Default|Get2))
  (Utilities|Array|Add _list (Variables|Default|Get3))
  (Utilities|Array|Add _list (Variables|Default|Get4)))

(event Collision|EventActorBeginOverlap
  (params (OtherActor :type Actor%20Object%20Reference)))

(event EventTick
  (params (DeltaSeconds :type Float%20%28single-precision%29)))

(fn ConstructionScript)

(fn ChangeMesh
  (params (Index :type Integer) (Material :type Material%20Interface%20Object%20Reference))
  (Rendering|Material|SetMaterial (Utilities|Array|Get(acopy) (Variables|Default|GetList) Index) 0 Material))