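; BP_VisualLobby is a lobby display that shows one skeletal mesh per player, with four slots.
; BeginPlay gathers the four mesh components into an ordered Players array.
; Tick polls NbPlayers on BP_GS_Lobby and, only when it differs from the cached count, unhides meshes below that index and hides the rest.
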(event EventBeginPlay
  (Utilities|Array|Add (Variables|Default|GetPlayers) (Variables|Default|GetSkeletalMesh1))
  (Utilities|Array|Add (Variables|Default|GetPlayers) (Variables|Default|GetSkeletalMesh2))
  (Utilities|Array|Add (Variables|Default|GetPlayers) (Variables|Default|GetSkeletalMesh3))
  (Utilities|Array|Add (Variables|Default|GetPlayers) (Variables|Default|GetSkeletalMesh4)))

(event EventTick
  (params (DeltaSeconds :type Float%20%28single-precision%29))
  (bind _asbp_gs_lobby (Utilities|Casting|CastToBP_GS_Lobby (Game|GetGameState)))
  (if (!= (Variables|/Game/Lobby/BP/BP_GS_Lobby.BP_GS_Lobby_C|GetNbPlayers _asbp_gs_lobby) (Variables|Default|GetNbPlayer))
    (bind _output_get (Variables|Default|SetNbPlayer (Variables|/Game/Lobby/BP/BP_GS_Lobby.BP_GS_Lobby_C|GetNbPlayers _asbp_gs_lobby)))
    (for (_array_element _array_index) (Variables|Default|GetPlayers)
      (Development|SetHiddeninGame _array_element (>= _array_index _output_get) false))))

(fn ConstructionScript)