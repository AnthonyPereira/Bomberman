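; Player character for a networked Bomberman-style game, handling skins, mount swap, bomb belt display and death.
; The authority derives the skin index from the object name, with an OnRep applying the material.
; A skill value toggles between Bomberman and Noupy-riding meshes through server and multicast events, while another sets visible belt bombs on Tick.
; Death launches and relocates the character unless the game has ended, when a surviving player's skin goes to the GameState podium.
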(event Custom|ChangeBomberman_multicast
  (CallFunction|SwitchtoDefault))

(event Custom|ChangeBomberman
  (Networking|SwitchHasAuthority
    (:Authority
      (CallFunction|ChangeBombermanMulticast))
    (:Remote
      (CallFunction|ChangeBombermanServer))))

(event Custom|ChangeMesh
  (Networking|SwitchHasAuthority
    (:Authority
      (CallFunction|ChangeMeshMulticast))
    (:Remote
      (CallFunction|ChangeMeshServer))))

(event Custom|ChangeBomberman_server
  (CallFunction|ChangeBombermanMulticast))

(event Custom|ChangeMesh_Server
  (CallFunction|ChangeMeshMulticast))

(event Custom|ChangeMesh_Multicast
  (CallFunction|SwitchtoNoopy))

(event EventBeginPlay
  (bind _self self)
  (bind _meshes (Variables|Default|GetMeshes))
  (bind _returnvalue (Utilities|GetObjectName _self))
  (bind _returnvalue_2 (Utilities|String|Len _returnvalue))
  (Input|DisableInput 0)
  (Utilities|FlowControl|Sequence
    (:then_0
      (Networking|SwitchHasAuthority
        (:Authority
          (Variables|Default|SetSkinIndex (Math|Conversions|ToInteger(Byte) (Utilities|String|GetSubstring _returnvalue (- _returnvalue_2 1) _returnvalue_2))))))
    (:then_1
      (Utilities|Casting|CastToPlayerController (Pawn|GetController))
      (Utilities|Array|Add _meshes (Variables|Default|GetBomb1))
      (Utilities|Array|Add _meshes (Variables|Default|GetBomb3))
      (Utilities|Array|Add _meshes (Variables|Default|GetBomb4))
      (Utilities|Array|Add _meshes (Variables|Default|GetBomb2))
      (Utilities|FlowControl|Delay 2.6)
      (Input|EnableInput 0))))

(event EventUpdateMyMesh
  (if (== (Variables|/Script/MyProject.Character_Skill|Getvalue (Utilities|Array|Get(acopy) (Variables|Default|GetList_Skills) 3)) 1)
    (CallFunction|ChangeMesh)
    (else
      (CallFunction|ChangeBomberman))))

(event EventDeath
  (bind _returnvalue (Transformation|GetActorLocation))
  (Input|DisableInput 0)
  (bind _asbp_my_project_player_controller (Utilities|Casting|CastToBP_MyProjectPlayerController (Pawn|GetController)))
  (bind _asbp_game_state (Utilities|Casting|CastToBP_GameState (Game|GetGameState)))
  (if (Variables|/Game/Blueprints/BP_GameState.BP_GameState_C|GetEndgame _asbp_game_state)
    (Variables|/Game/Blueprints/BP_MyProjectPlayerController.BP_MyProjectPlayerController_C|SetAlive _asbp_my_project_player_controller true)
    (else
      (Variables|/Game/Blueprints/BP_MyProjectPlayerController.BP_MyProjectPlayerController_C|SetAlive _asbp_my_project_player_controller false)
      (Collision|SetCollisionEnabled (Variables|Default|GetCapsuleComponent) "NoCollision")
      (Utilities|Casting|CastToBP_GameState (Game|GetGameState))
      (bind _returnvalue_2 (Effects|SpawnEmitterAttached "/Game/Particle/Smoke.Smoke" (Variables|Character|GetMesh) "None" "0, 0, 0" "0, 0,180.000000" "2.000000,2.000000,2.000000"))
      (Character|LaunchCharacter (Math|Vector|MakeVector (* (.x _returnvalue) 2.0) (* (.y _returnvalue) 2.0) 1.2e+03) true false)
      (Utilities|FlowControl|Delay 1.5)
      (Components|DestroyComponent _returnvalue_2)
      (Collision|SetCollisionEnabled (Variables|Default|GetCapsuleComponent) "QueryAndPhysics")
      (Transformation|SetActorLocation "-2500.000000,0.000000,60.000000" false false))))

(event EventTick
  (params (DeltaSeconds :type Float%20%28single-precision%29))
  (Utilities|FlowControl|Sequence
    (:then_0
      (for (_array_element _array_index) (Variables|Default|GetMeshes)
        (Development|SetHiddeninGame _array_element (not (< _array_index (Variables|/Script/MyProject.Character_Skill|Getvalue (Utilities|Array|Get(acopy) (Variables|Default|GetList_Skills) 1)))) false)))
    (:then_1
      (bind _asbp_my_project_player_controller (Utilities|Casting|CastToBP_MyProjectPlayerController (Pawn|GetController)))
      (bind _asbp_game_state (Utilities|Casting|CastToBP_GameState (Game|GetGameState)))
      (if (and (Variables|/Game/Blueprints/BP_GameState.BP_GameState_C|GetEndgame _asbp_game_state) (Variables|/Game/Blueprints/BP_MyProjectPlayerController.BP_MyProjectPlayerController_C|GetAlive _asbp_my_project_player_controller))
        (Utilities|FlowControl|DoOnce false
          (:Completed
            (Variables|/Game/Blueprints/BP_GameState.BP_GameState_C|SetPodium _asbp_game_state (Utilities|Array|Get(acopy) (Variables|Default|GetMaterial) (Variables|Default|GetSkinIndex)))))))))

(fn ConstructionScript)

(fn OnRepSkin
  (bind _material (Variables|Default|GetMaterial))
  (bind _skinindex (Variables|Default|GetSkinIndex))
  (bind _output (Utilities|Array|Get(acopy) _material _skinindex))
  (Rendering|Material|SetMaterial (Variables|Character|GetMesh) 0 _output)
  (Rendering|Material|SetMaterial (Variables|Default|GetRidding) 0 _output))

(fn SwitchtoNoopy
  (bind _mesh (Variables|Character|GetMesh))
  (Class|SkinnedMeshComponent|SetSkeletalMesh _mesh "/Game/BombermanMannequin/Noopy/Noupy.Noupy" true)
  (Rendering|Material|SetMaterial _mesh 0 "/Game/BombermanMannequin/Noopy/M_Noupy.M_Noupy")
  (Transformation|SetWorldScale3D _mesh "0.220000,0.220000,0.220000")
  (Class|SkeletalMeshComponent|SetAnimClass (Variables|Character|GetMesh) "/Game/BombermanMannequin/Noopy/BP_AnimNoupy.BP_AnimNoupy_C")
  (Development|SetHiddeninGame (Variables|Default|GetRidding) false false))

(fn SwitchtoDefault
  (bind _mesh (Variables|Character|GetMesh))
  (Class|SkinnedMeshComponent|SetSkeletalMesh _mesh "/Game/BombermanMannequin/bomberman2.bomberman2" true)
  (Rendering|Material|SetMaterial _mesh 0 (Utilities|Array|Get(acopy) (Variables|Default|GetMaterial) (Variables|Default|GetSkinIndex)))
  (Transformation|SetWorldScale3D _mesh "0.500000,0.500000,0.500000")
  (Class|SkeletalMeshComponent|SetAnimClass (Variables|Character|GetMesh) "/Game/BombermanMannequin/Animation/BP_AnimBomberman.BP_AnimBomberman_C")
  (Development|SetHiddeninGame (Variables|Default|GetRidding) true false))

(fn HideBombBelt
  (for _array_element (Variables|Default|GetMeshes)
    (Development|SetHiddeninGame _array_element true false)))