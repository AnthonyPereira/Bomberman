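; Player controller for the main menu, which shows the menu HUD widget and handles hosting and joining games.
; On BeginPlay it adds BP_HUD_Menu to the viewport, shows the cursor and sets Game and UI input mode.
; Host creates a non-LAN session and, on success, opens the Lobby level as a listen server.
; Join runs an "open" console command with the supplied address string appended.
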(event Custom|HUD%20-%20Menu
  ;[1 1 1] HUD Menu
  (bind _returnvalue (UserInterface|CreateWidget "/Game/Menu/HUD/BP_HUD_Menu.BP_HUD_Menu_C" self))
  (UserInterface|Viewport|AddtoViewport _returnvalue 0))

(event Custom|init_cursor
  ;[1 1 1] Init Cursor
  (Variables|Default|SetbShowMouseCursor true)
  (Input|SetInputModeGameandUI self 0 "DoNotLock" false))

(event Custom|Host
  (|Session self 4 false
    (:OnSuccess
      (Game|OpenLevel(byName) "Lobby" true "listen"))))

(event Custom|Join
  (params (B :type String))
  (Development|ExecuteConsoleCommand (Utilities|String|Append "open " B) 0))

(event EventBeginPlay
  ;[1 1 1] Init
  (CallFunction|HUD-Menu)
  (CallFunction|InitCursor))

(fn ConstructionScript)