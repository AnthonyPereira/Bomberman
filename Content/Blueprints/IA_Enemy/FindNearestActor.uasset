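; Behavior tree task that stores the location of the player character nearest to the controlled pawn in the NearestEnemy blackboard key.
; After a delay, it gathers all BP_PlayerCharacter actors, removes the pawn itself and picks the nearest by distance.
; It prints a debug string and finishes successfully after another short delay.
; A pawn that fails the BP_PlayerCharacter cast never reaches FinishExecute.
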(event EventReceiveExecuteAI
  (params (OwnerController :type AI%20Controller%20Object%20Reference) (ControlledPawn :type Pawn%20Object%20Reference))
  (Utilities|FlowControl|Delay 2.0)
  (bind _asbp_player_character (Utilities|Casting|CastToBP_PlayerCharacter ControlledPawn))
  (bind _outactors (Actor|GetAllActorsOfClass "/Game/Blueprints/BP_PlayerCharacter.BP_PlayerCharacter_C"))
  (bind _output_get (Variables|Default|SetOut%20Actors _outactors))
  (Utilities|Array|RemoveItem _output_get _asbp_player_character)
  (Development|PrintString "Hello")
  (AI|BehaviorTree|SetBlackboardValueasVector (Variables|Default|GetNearestEnemy) (Transformation|GetActorLocation (.ReturnValue (Actor|FindNearestActor (Transformation|GetActorLocation ControlledPawn) _output_get))))
  (Utilities|FlowControl|Delay 0.1)
  (AI|BehaviorTree|FinishExecute true))